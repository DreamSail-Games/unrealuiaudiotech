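; A music player actor that hosts an in-world widget and can be picked up by BP_MotionController.
; On BeginPlay it casts the widget component's object to MusicPlayerWidget, binds its SongPlayed event and initializes it.
; Each song the widget reports is set on the Audio component and played.
; Pickup and Drop attach and detach the actor keeping world transform, both disabling physics on the Cube.
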(event `self.ReceiveBeginPlay`
  (bind _asmusic_player_widget (cast `/Game/Menus/MusicPlayerWidget` (`WidgetComponent.GetUserWidgetObject` (`self.Widget`)))
    (:`then`
      (add `/Game/Menus/MusicPlayerWidget.SongPlayed` _asmusic_player_widget (delegate `SongPlayed_Event_0`))
      (`/Game/Menus/MusicPlayerWidget.Initialize` _asmusic_player_widget)
      (`KismetSystemLibrary.PrintString` "Music player intialize"))
    (:`CastFailed`
      (`KismetSystemLibrary.PrintString` "Hello"))))

(event `SongPlayed_Event_0`
  (params (SongPlayed :type "SoundWave Object Reference"))
  (bind _audio (`self.Audio`))
  (`AudioComponent.SetSound` _audio SongPlayed)
  (`AudioComponent.Play` _audio 0.0)
  (`KismetSystemLibrary.PrintString` "Very Top level audio play"))

(event `/Game/VirtualRealityBP/Blueprints/PickupActorInterface.Pickup`
  (params (AttachTo :type "SceneComponent Object Reference"))
  (`PrimitiveComponent.SetSimulatePhysics` (`self.Cube`) false)
  (`SceneComponent.K2_AttachToComponent` (`self.K2_GetRootComponent`) AttachTo "None" "KeepWorld" "KeepWorld" "KeepWorld" false))

(event `/Game/VirtualRealityBP/Blueprints/PickupActorInterface.Drop`
  (`PrimitiveComponent.SetSimulatePhysics` (`self.Cube`) false)
  (`self.K2_DetachFromActor` "KeepWorld" "KeepWorld" "KeepWorld"))

(fn `UserConstructionScript`)